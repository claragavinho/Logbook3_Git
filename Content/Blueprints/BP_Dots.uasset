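; BP_Dots is a collectable dot that the third-person character picks up by touching its sphere.
; On overlap it adds points to the character's Score, then calls AdjustCollectables.
; That function decrements CollectablesLeft on the third-person game mode, adds a newly created WBP_Collectables widget to the viewport on every pickup, and destroys the dot.
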(event OnComponentBeginOverlap(Sphere)
  (params (OverlappedComponent :type Primitive%20Component%20Object%20Reference) (OtherActor :type Actor%20Object%20Reference) (OtherComp :type Primitive%20Component%20Object%20Reference) (OtherBodyIndex :type Integer) (bFromSweep :type Boolean) (SweepResult :type Hit%20Result%20Structure%20%28by%20ref%29))
  (bind _asbp_third_person_character (Utilities|Casting|CastToBP_ThirdPersonCharacter OtherActor))
  (Variables|/Game/ThirdPerson/Blueprints/BP_ThirdPersonCharacter.BP_ThirdPersonCharacter_C|SetScore _asbp_third_person_character (+ (Variables|/Game/ThirdPerson/Blueprints/BP_ThirdPersonCharacter.BP_ThirdPersonCharacter_C|GetScore _asbp_third_person_character) 10))
  (CallFunction|AdjustCollectables))

(fn ConstructionScript)

(fn AdjustCollectables
  (bind _asbp_third_person_game_mode (Utilities|Casting|CastToBP_ThirdPersonGameMode (Game|GetGameMode)))
  (bind _result (Math|Integer|DecrementInt (Variables|/Game/ThirdPerson/Blueprints/BP_ThirdPersonGameMode.BP_ThirdPersonGameMode_C|GetCollectablesLeft _asbp_third_person_game_mode))
    (:%20%20
      (Variables|/Game/ThirdPerson/Blueprints/BP_ThirdPersonGameMode.BP_ThirdPersonGameMode_C|SetCollectablesLeft _asbp_third_person_game_mode _result)
      (bind _returnvalue (UserInterface|CreateWidget "/Game/Blueprints/WBP_Collectables.WBP_Collectables_C"))
      (UserInterface|Viewport|AddtoViewport _returnvalue 0)
      (Actor|DestroyActor))))